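; BP_Cannon is a cannon actor whose CannonComponent pitches to an open angle and back to zero on demand.
; CannonRotator and CannonRotatorReverse each play their own timeline from the start, driving the component's relative pitch toward OpenAngle or zero, with roll and yaw held at zero.
; Each update lerps from the current pitch rather than a stored start value, so the motion compounds instead of following the timeline curve linearly.
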(event EventCannonRotatorReverse
  (bind _rotar (Timeline|Timeline_1 PlayFromStart)
    (:Update
      (Transformation|SetRelativeRotation (Variables|Default|GetCannonComponent) (Math|Rotator|MakeRotator 0.0 (Math|Float|Lerp (.Pitch (Math|Rotator|BreakRotator (Variables|/Script/Engine.SceneComponent|GetRelativeRotation (Variables|Default|GetCannonComponent)))) 0.0 _rotar) 0.0) false false))))

(event Collision|EventActorBeginOverlap
  (params (OtherActor :type Actor%20Object%20Reference)))

(event EventTick
  (params (DeltaSeconds :type Float%20%28single-precision%29)))

(event EventCannonRotator
  (bind _rotar (Timeline|Timeline_0 PlayFromStart)
    (:Update
      (Transformation|SetRelativeRotation (Variables|Default|GetCannonComponent) (Math|Rotator|MakeRotator 0.0 (Math|Float|Lerp (.Pitch (Math|Rotator|BreakRotator (Variables|/Script/Engine.SceneComponent|GetRelativeRotation (Variables|Default|GetCannonComponent)))) (Variables|Default|GetOpenAngle) _rotar) 0.0) false false))))

(fn ConstructionScript)